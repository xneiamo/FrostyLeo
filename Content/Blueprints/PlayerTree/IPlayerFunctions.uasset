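; IPlayerFunctions is, by its name and stub functions, a Blueprint interface for querying the player character's movement state.
; It declares boolean getters for falling, moving, running, jumping, jump peak, crouching and facing right.
; Each graph here is a placeholder returning false and holds no logic of its own.
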(fn `F_IsCrouching`
  (returns (Out :type Boolean))
  (return false))

(fn `F_IsFacingRight`
  (returns (Out :type Boolean))
  (return false))

(fn `F_IsFalling`
  (returns (bIsFalling :type Boolean))
  (return false))

(fn `F_IsJumping`
  (returns (Out :type Boolean))
  (return false))

(fn `F_IsMoving`
  (returns (bIsMoving :type Boolean))
  (return false))

(fn `F_IsPeakJump`
  (returns (Out :type Boolean))
  (return false))

(fn `F_IsRunning`
  (returns (Out :type Boolean))
  (return false))