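; AbstractPlayer is a base player Blueprint that tracks movement and pose flags such as falling, running, jumping, crouching and facing right.
; UpdateState refreshes each flag through its own query function, then writes them all into the State struct.
; Most queries echo the stored flag, while the moving query always returns false.
; Setter and toggle events change flags directly; jump input checks CanJump, and crouch input is an empty stub.
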(event `UpdateState`
  (`self.F_UpdateState`))

(event `SetIsFacingRight`
  (params (Input :type Boolean :default false))
  (set `self.IsFacingRight` Input))

(event `SetIsJumping`
  (params (Input :type Boolean :default false))
  (set `self.IsJumping` Input))

(event `SetIsPeakJump`
  (params (Input :type Boolean :default false))
  (set `self.IsPeakJump` Input))

(event `SetIsRunning`
  (params (Input :type Boolean :default false))
  (set `self.IsRunning` Input))

(event `SetIsFalling`
  (params (Input :type Boolean :default false))
  (set `self.IsFalling` Input))

(event `SetIsCrouching`
  (params (Input :type Boolean :default false))
  (set `self.IsCrouching` Input))

(event `SetIsMoving`
  (params (Input :type Boolean :default false))
  (set `self.IsMoving` Input))

(event `ToggleIsFacingRight`
  (`self.SetIsFacingRight` (not (`self.IsFacingRight`))))

(event `ToggleIsJumping`
  (`self.SetIsJumping` (not (`self.IsJumping`))))

(event `ToggleIsPeakJump`
  (`self.SetIsPeakJump` (not (`self.IsPeakJump`))))

(event `ToggleIsRunning`
  (`self.SetIsRunning` (not (`self.IsRunning`))))

(event `ToggleIsFalling`
  (`self.SetIsFalling` (not (`self.IsFalling`))))

(event `ToggleIsCrouching`
  (`self.SetIsCrouching` (not (`self.IsCrouching`))))

(event `ToggleIsMoving`
  (`self.SetIsMoving` (not (`self.IsMoving`))))

(fn `F_IsCrouching`
  (returns (Out :type Boolean))
  (return (`self.IsCrouching`)))

(fn `F_IsFacingRight`
  (returns (Out :type Boolean))
  (return (`self.IsFacingRight`)))

(fn `F_IsFalling`
  (returns (bIsFalling :type Boolean))
  (return (`self.IsFalling`)))

(fn `F_IsJumping`
  (returns (Out :type Boolean))
  (return (`self.IsJumping`)))

(fn `F_IsMoving`
  (returns (bIsMoving :type Boolean))
  (return false))

(fn `F_IsPeakJump`
  (returns (Out :type Boolean))
  (return (`self.IsPeakJump`)))

(fn `F_IsRunning`
  (returns (Out :type Boolean))
  (return (`self.IsRunning`)))

(fn `F_UpdateState`
  (bind _bisfalling (`self.F_IsFalling`))
  (bind _output_get (set `self.IsFalling` _bisfalling))
  (bind _bismoving (`self.F_IsMoving`))
  (bind _output_get_2 (set `self.IsMoving` _bismoving))
  (bind _out (`self.F_IsRunning`))
  (bind _output_get_3 (set `self.IsRunning` _out))
  (bind _out_2 (`self.F_IsPeakJump`))
  (bind _output_get_4 (set `self.IsPeakJump` _out_2))
  (bind _out_3 (`self.F_IsJumping`))
  (bind _output_get_5 (set `self.IsJumping` _out_3))
  (bind _out_4 (`self.F_IsFacingRight`))
  (bind _output_get_6 (set `self.IsFacingRight` _out_4))
  (bind _out_5 (`self.F_IsCrouching`))
  (bind _output_get_7 (set `self.IsCrouching` _out_5))
  (setmembers `/Game/Blueprints/PlayerTree/PlayerState` :`StructRef` (`self.State`) :`IsFalling` _output_get :`IsMoving` _output_get_2 :`IsRunning` _output_get_3 :`IsPeakJump` _output_get_4 :`IsJumping` _output_get_5 :`FacingRight` _output_get_6 :`IsCrouching` _output_get_7))

(fn `InputCrouch`)

(fn `InputJump`
  (if (`self.CanJump`)
    (`self.Jump`)
    (return)))

(fn `UserConstructionScript`)