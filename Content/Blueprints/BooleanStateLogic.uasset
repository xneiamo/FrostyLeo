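; BooleanStateLogic is a utility library of boolean and range-comparison helpers.
; Between and BetweenEqual report high, in-range and low flags with strict or inclusive bounds, and BooleanSwitch returns a value alongside its inverse.
; IncrementIfDifferent uses BetweenEqual to output one when two values differ beyond a tolerance.
; KeyCount looks like an unfinished timer-based counter: it only schedules a debug print, and its counting nodes are disconnected.
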(fn Between
  (params (HighValue :type Float%20%28single-precision%29 :default 0.0) (InputValue :type Float%20%28single-precision%29 :default 0.0) (LowValue :type Float%20%28single-precision%29 :default 0.0))
  (bind _returnvalue (> InputValue LowValue))
  (bind _returnvalue_2 (> HighValue InputValue))
  (return (not _returnvalue_2) (and _returnvalue_2 _returnvalue) (not _returnvalue)))

(fn BooleanSwitch
  (params (Input :type Boolean :default false))
  (return Input (not Input)))

(fn KeyCount
  (params (NewParam :type Object%20Object%20Reference))
  (if (not (Class|KismetSystemLibrary|TimerExists NewParam "KeyCount"))
    (Development|PrintString 0 "False")
    (Utilities|Time|SetTimerbyFunctionName NewParam "PrintCount" 1.0)))

(fn PrintCount
  (Development|PrintString 0))

(fn IncrementifDifferent
  (params (LastValue :type Float%20%28single-precision%29 :default 0.0) (CurrentValue :type Float%20%28single-precision%29 :default 0.0) (Tolerance :type Float%20%28single-precision%29 :default 0.0))
  (bind _isbetween (CallFunction|BetweenEqual (+ CurrentValue Tolerance) LastValue (- CurrentValue Tolerance)))
  (if _isbetween
    (LocalVariables|SetOutputValue 0.0)
    (else
      (LocalVariables|SetOutputValue 1.0)))
  (return (LocalVariables|GetOutputValue)))

(fn BetweenEqual
  (params (HighValue :type Float%20%28single-precision%29 :default 0.0) (InputValue :type Float%20%28single-precision%29 :default 0.0) (LowValue :type Float%20%28single-precision%29 :default 0.0))
  (bind _returnvalue (>= InputValue LowValue))
  (bind _returnvalue_2 (>= HighValue InputValue))
  (return (not _returnvalue_2) (and _returnvalue_2 _returnvalue) (not _returnvalue)))